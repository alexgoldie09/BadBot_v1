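; Player-controlled flying bot pawn with twin rifle blasters, driven by Enhanced Input.
; Move input feeds FloatingPawnMovement along the control rotation's right, forward and up axes, giving full three-axis flight.
; Look input drives controller yaw and pitch, and Tick snaps the bot mesh to the control rotation.
; Fire spawns blaster bolts from both rifle sockets at once, or alternates left and right through a FlipFlop when Alternatefire is set.
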(event `EnhancedInput|/Game/Blueprints/Input/InputActions/IA_Fire`
  (params (ActionValue :type Boolean) (ElapsedSeconds :type "Float (double-precision)") (TriggeredSeconds :type "Float (double-precision)") (InputAction :type "InputAction Object Reference" :default "/Game/Blueprints/Input/InputActions/IA_Fire.IA_Fire"))
  ;[0.15 0 0 0.5] Shooting
  (:`Triggered`
    (if (`self.bAlternatefire`)
      (`/Engine/EditorBlueprintResources/StandardMacros.FlipFlop`
        (:`A`
          (`self.SpawnBlasterBolt` (`self.SocketRifleL`)))
        (:`B`
          (`self.SpawnBlasterBolt` (`self.SocketRifleR`))))
      (else
        (`self.SpawnBlasterBolt` (`self.SocketRifleL`))
        (`self.SpawnBlasterBolt` (`self.SocketRifleR`))))))

(event `EnhancedInput|/Game/Blueprints/Input/InputActions/IA_Look`
  (params (ActionValue :type "Vector2D Structure") (ElapsedSeconds :type "Float (double-precision)") (TriggeredSeconds :type "Float (double-precision)") (InputAction :type "InputAction Object Reference" :default "/Game/Blueprints/Input/InputActions/IA_Look.IA_Look"))
  ;[0.15 0.1157 0 0.5] Look Around
  (:`Triggered`
    (`self.HandleLookAround` ActionValue)))

(event `EnhancedInput|/Game/Blueprints/Input/InputActions/IA_Move`
  (params (ActionValue :type "Vector Structure") (ElapsedSeconds :type "Float (double-precision)") (TriggeredSeconds :type "Float (double-precision)") (InputAction :type "InputAction Object Reference" :default "/Game/Blueprints/Input/InputActions/IA_Move.IA_Move"))
  ;[0.15 0.7449 0.15 0.5] Move Around
  (:`Triggered`
    (`self.HandleFloatingPawnMovement`)))

(event `self.ReceiveTick`
  (params (DeltaSeconds :type "Float (single-precision)"))
  (`SceneComponent.K2_SetWorldRotation` (`self.BotMesh`) (`self.GetControlRotation`) false false))

(fn `GetForwardInput`
  (returns (ReturnValue :type "Vector Structure"))
  (return (* (.y (`|GetInputActionValue`)) (`KismetMathLibrary.GetForwardVector` (`self.GetControlRotation`)))))

(fn `GetRightInput`
  (returns (ReturnValue :type "Vector Structure"))
  (return (* (`KismetMathLibrary.GetRightVector` (`self.GetControlRotation`)) (.x (`|GetInputActionValue`)))))

(fn `GetUpInput`
  (returns (ReturnValue :type "Vector Structure"))
  (return (* (`KismetMathLibrary.GetUpVector` (`self.GetControlRotation`)) (.z (`|GetInputActionValue`)))))

(fn `HandleFloatingPawnMovement`
  (`PawnMovementComponent.AddInputVector` (`self.FloatingPawnMovement`) (`self.GetRightInput`) false)
  (`PawnMovementComponent.AddInputVector` (`self.FloatingPawnMovement`) (`self.GetForwardInput`) false)
  (`PawnMovementComponent.AddInputVector` (`self.FloatingPawnMovement`) (`self.GetUpInput`) false))

(fn `HandleLookAround`
  (params (ActionValue :type "Vector2D Structure"))
  (bind (_x _y) (`KismetMathLibrary.BreakVector2D` ActionValue))
  (`self.AddControllerYawInput` _x)
  (`self.AddControllerPitchInput` _y))

(fn `UserConstructionScript`)