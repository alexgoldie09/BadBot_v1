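; BP_Pickup is a short-lived score pickup that increments the BP_BadBotGameMode score when a Pawn overlaps its sphere volume.
; A timeline scales the mesh in on spawn, and either overlap or the lifetime timer triggers a guarded scale-out that destroys the actor.
; Each tick moves it along its forward vector while a random spin rotates the actor, continually changing its heading.
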(event `WinkIn`
  ;[0.15 0 0.09166 0.5] Start WinkIn Timeline
  (bind (_direction _scale) (`Timeline|WinkIn Timeline`)
    (:`Update`
      (`SceneComponent.SetWorldScale3D` (`self.SphereMesh`) _scale))))

(event `self.ReceiveBeginPlay`
  (`self.WinkIn`)
  (`self.InitDeltaRotation`)
  ;[0.15 0.01596 0.07835 0.5] Start WinkOut Timeline
  (`KismetSystemLibrary.K2_SetTimerDelegate` (delegate `WinkOut`) (`self.Lifetime`))
  (add `PrimitiveComponent.OnComponentBeginOverlap` (`self.SphereVolume`) (delegate `OnPickupOverlap`)))

(event `OnPickupOverlap`
  (params (OverlappedComponent :type "PrimitiveComponent Object Reference") (OtherActor :type "Actor Object Reference") (OtherComp :type "PrimitiveComponent Object Reference") (OtherBodyIndex :type Integer) (bFromSweep :type Boolean) (SweepResult :type "HitResult Structure (by ref)"))
  ;[0.15 0.01596 0.07835 0.5] Start WinkOut Timeline
  (if (`GameplayStatics.ObjectIsA` OtherActor "/Script/Engine.Pawn")
    (bind _asbp_bad_bot_game_mode (cast `/Game/Blueprints/Game/BP_BadBotGameMode` (`GameplayStatics.GetGameMode`)))
    (`BadBotGameMode.IncrementScore` _asbp_bad_bot_game_mode)
    (`self.WinkOut`)))

(event `WinkOut`
  ;[0.15 0.01596 0.07835 0.5] Start WinkOut Timeline
  (if (not (`self.IsWinking`))
    (set `self.IsWinking` true)
    (bind (_direction _scale) (`Timeline|WinkOutTimeline`)
      (:`Update`
        (`self.ScaleSphere` _scale))
      (:`Finished`
        (`self.K2_DestroyActor`)))))

(event `self.ReceiveTick`
  (params (DeltaSeconds :type "Float (single-precision)"))
  ;[0.04587 0.15 0.1154 0.5] Update Location & Rotation
  (`self.UpdateLocation`)
  (`self.UpdateRotation`))

(fn `InitDeltaRotation`
  (set `self.DeltaRot` (* (`KismetMathLibrary.RandomRotator` false) (`self.RotScale`))))

(fn `ScaleSphere`
  (params (Scale :type "Float (single-precision)"))
  (`SceneComponent.SetWorldScale3D` (`self.SphereMesh`) (`KismetMathLibrary.MakeVector` Scale Scale Scale)))

(fn `UpdateLocation`
  (`self.K2_AddActorWorldOffset` (* (* (`GameplayStatics.GetWorldDeltaSeconds`) (`self.Speed`)) (`self.GetActorForwardVector`))))

(fn `UpdateRotation`
  (`self.K2_AddActorWorldRotation` (* (`self.DeltaRot`) (`GameplayStatics.GetWorldDeltaSeconds`))))

(fn `UserConstructionScript`)